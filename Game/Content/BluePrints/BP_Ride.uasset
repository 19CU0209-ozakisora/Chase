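; BP_Ride is a ride zone that tracks a BP_Chair's progress between a start point and an end point.
; Its collision captures the chair and flags it as riding; on exit, a chair without ride input is stopped and set to the end phase.
; During the ride phase, Tick feeds a 2D distance ratio into the chair's speed percent, zeroed at or past full length, with debug printing.
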(event OnComponentBeginOverlap(CollisionComponent)
  (params (OverlappedComponent :type Primitive%20Component%20Object%20Reference) (OtherActor :type Actor%20Object%20Reference) (OtherComp :type Primitive%20Component%20Object%20Reference) (OtherBodyIndex :type Integer) (bFromSweep :type Boolean) (SweepResult :type Hit%20Result%20Structure%20%28by%20ref%29))
  (bind _asbp_chair (Utilities|Casting|CastToBP_Chair OtherActor))
  (bind _output_get (Variables|Default|Setcontrol_chair _asbp_chair))
  (Variables|/Script/Chase.Chair|Setm_in_ride_flag_ _output_get true))

(event OnComponentEndOverlap(CollisionComponent)
  (params (OverlappedComponent :type Primitive%20Component%20Object%20Reference) (OtherActor :type Actor%20Object%20Reference) (OtherComp :type Primitive%20Component%20Object%20Reference) (OtherBodyIndex :type Integer))
  (bind _control_chair (Variables|Default|Getcontrol_chair))
  (if (== OtherActor _control_chair)
    (Variables|/Script/Chase.Chair|Setm_in_ride_flag_ _control_chair false)
    (if (Variables|/Script/Chase.Chair|Getm_is_input_ride_ _control_chair)
      _
      (else
        (Variables|/Script/Engine.FloatingPawnMovement|SetMaxSpeed (Variables|/Script/Chase.Chair|Getm_floating_pawn_movement_ _control_chair) 0.0)
        (Class|Chair|SetPhase _control_chair "kEnd"))))
  (Utilities|FlowControl|Delay 2.0)
  (Variables|Default|Setleap 0.0))

(event EventBeginPlay)

(event Collision|EventActorBeginOverlap
  (params (OtherActor :type Actor%20Object%20Reference)))

(event EventTick
  (params (DeltaSeconds :type Float%20%28single-precision%29))
  (bind _control_chair (Variables|Default|Getcontrol_chair))
  (bind _startpoint (Variables|Default|GetStartPoint))
  (bind _endpoint (Variables|Default|GetEndPoint))
  (bind _returnvalue (Transformation|GetWorldLocation _endpoint))
  (bind _returnvalue_2 (Transformation|GetActorLocation _control_chair))
  (bind _returnvalue_3 (Transformation|GetWorldLocation _startpoint))
  (bind _output_get (Variables|Default|Setstart_pos (Math|Vector2D|MakeVector2D (.x _returnvalue_3) (.y _returnvalue_3))))
  (bind _output_get_2 (Variables|Default|Setend_pos (Math|Vector2D|MakeVector2D (.x _returnvalue) (.y _returnvalue))))
  (if (Utilities|IsValid _control_chair)
    (bind _returnvalue_4 (Class|Chair|GetPhase _control_chair))
    (if (Utilities|Enum|Equal(Enum) _returnvalue_4 "kRide")
      (bind _output_get_3 (Variables|Default|Setplayer_pos (Math|Vector2D|MakeVector2D (.x _returnvalue_2) (.y _returnvalue_2))))
      (Development|PrintString (Utilities|String|ToString(Float) (/ (Math|Vector|Distance2D(Vector) (Variables|Default|Getstart_pos) _output_get_3) (Math|Vector|Distance2D(Vector) _output_get _output_get_2))) true true "(R=0.000000,G=0.660000,B=1.000000,A=1.000000)" (Utilities|Time|GetWorldDeltaSeconds))
      (bind _output_get_4 (Variables|Default|Setleap (/ (Math|Vector|Distance2D(Vector) (Variables|Default|Getstart_pos) _output_get_3) (Math|Vector|Distance2D(Vector) _output_get _output_get_2))))
      (if (< _output_get_4 1.0)
        (Development|PrintString (Utilities|String|Append "% = " (Utilities|String|ToString(Float) _output_get_4)) true false "(R=1.000000,G=0.684933,B=0.000000,A=1.000000)" DeltaSeconds)
        (else
          (bind _output_get_5 (Variables|Default|Setleap 0.0))
          (Development|PrintString (Utilities|String|Append "% = " (Utilities|String|ToString(Float) _output_get_5)) true false "(R=1.000000,G=0.684933,B=0.000000,A=1.000000)" DeltaSeconds)))
      (Variables|/Script/Chase.Chair|Setm_speed_percent_ (Variables|Default|Getcontrol_chair) (Variables|Default|Getleap)))))

(fn ConstructionScript)