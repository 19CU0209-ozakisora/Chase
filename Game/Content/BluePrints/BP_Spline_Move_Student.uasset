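; Spline-following actor that moves a skeletal mesh continuously along its spline, by its name a student character.
; Each Tick advances a travelled distance by Speed times delta time and samples world location and rotation through GetCurrentLocation, which wraps distance by spline length to loop.
; The mesh is teleported to that transform with a yaw offset added.
; Helper functions for spline length and arrival are defined but unused here.
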(event EventBeginPlay)

(event Collision|EventActorBeginOverlap
  (params (OtherActor :type Actor%20Object%20Reference)))

(event EventTick
  (params (DeltaSeconds :type Float%20%28single-precision%29))
  (bind _output_get (Variables|Default|SetLocalLength (+ (* DeltaSeconds (Variables|Default|GetSpeed)) (Variables|Default|GetLocalLength))))
  (bind (_location _rotation) (CallFunction|GetCurrentLocation _output_get true))
  (Transformation|SetWorldLocationAndRotation (Variables|Default|GetSkeletalMesh) _location (Math|Rotator|MakeRotator (.roll _rotation) (.pitch _rotation) (+ (.yaw _rotation) (Variables|Default|GetRotation_OFFSET))) false true))

(fn ConstructionScript)

(fn GetCurrentLocation
  (params (Length :type Float%20%28single-precision%29) (Loop :type Boolean))
  (bind _spline (Variables|Default|GetSpline))
  (if Loop
    (Variables|Default|SetLocalLength (Math|Float|%(Float) Length (Spline|GetSplineLength (Variables|Default|GetSpline))))
    (else
      (Variables|Default|SetLocalLength Length)))
  (return (Spline|GetLocationatDistanceAlongSpline _spline (Variables|Default|GetLocalLength) "World") (Spline|GetRotationatDistanceAlongSpline _spline (Variables|Default|GetLocalLength) "World")))

(fn GetSplineLength
  (return (Spline|GetSplineLength (Variables|Default|GetSpline))))

(fn IsArrived
  (params (Length :type Float%20%28single-precision%29))
  (return (>= Length (Spline|GetSplineLength (Variables|Default|GetSpline)))))