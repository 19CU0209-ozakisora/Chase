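; BP_PlayerCharacter is the player character Blueprint, which prints Japanese keyboard instructions at BeginPlay: arrows to turn, Enter to confirm.
; Pressing Enter destroys its StaticMesh component after a validity check.
; When that mesh hits an actor tagged "Stone", it prints a debug message and sets SpeedScale to zero.
; The graph holds no turning logic, and Tick, overlap and construction script are empty.
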(event OnComponentHit(StaticMesh)
  (params (HitComponent :type Primitive%20Component%20Object%20Reference) (OtherActor :type Actor%20Object%20Reference) (OtherComp :type Primitive%20Component%20Object%20Reference) (NormalImpulse :type Vector :default "0, 0, 0") (Hit :type Hit%20Result%20Structure%20%28by%20ref%29))
  (if (Actor|ActorHasTag OtherActor "Stone")
    (Development|PrintString "Stone Hit")
    (Variables|Default|Setspeed_scale_ 0.0)))

(event EventBeginPlay
  (Development|PrintString "キーボード操作のみ 
 
← or→ で向きの変更 
Enterで決定"))

(event Collision|EventActorBeginOverlap
  (params (OtherActor :type Actor%20Object%20Reference)))

(event EventTick
  (params (DeltaSeconds :type Float%20%28single-precision%29)))

(event Input|KeyboardEvents|Enter
  (params (Key :type Key%20Structure :default "None"))
  (bind _staticmesh (Variables|Default|GetStaticMesh))
  ;[1 1 1] スタティックメッシュのNULLチェック後削除
  (:Pressed
    (if (Utilities|IsValid _staticmesh)
      (Components|DestroyComponent _staticmesh))))

(fn ConstructionScript)