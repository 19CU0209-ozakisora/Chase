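; BP_OutZone is a zone Blueprint that disables collision on actors that come to rest inside its Cube volume.
; Swept overlaps on the Cube add actors to DeleteActorArray, and end overlaps remove them.
; Tick prints the array count and passes actors with near-zero velocity to ActorDelete.
; Despite its name, ActorDelete only disables collision and untracks the actor; its gravity-disabling branch is unconnected.
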(event OnComponentBeginOverlap(Cube)
  (params (OverlappedComponent :type Primitive%20Component%20Object%20Reference) (OtherActor :type Actor%20Object%20Reference) (OtherComp :type Primitive%20Component%20Object%20Reference) (OtherBodyIndex :type Integer) (bFromSweep :type Boolean) (SweepResult :type Hit%20Result%20Structure%20%28by%20ref%29))
  (if bFromSweep
    (Utilities|Array|AddUnique (Variables|Default|GetdeleteActorArray) OtherActor)))

(event OnComponentEndOverlap(Cube)
  (params (OverlappedComponent :type Primitive%20Component%20Object%20Reference) (OtherActor :type Actor%20Object%20Reference) (OtherComp :type Primitive%20Component%20Object%20Reference) (OtherBodyIndex :type Integer))
  (if (Utilities|Array|ContainsItem (Variables|Default|GetdeleteActorArray) OtherActor)
    (Utilities|Array|RemoveItem (Variables|Default|GetdeleteActorArray) OtherActor)))

(event EventBeginPlay)

(event Collision|EventActorBeginOverlap
  (params (OtherActor :type Actor%20Object%20Reference)))

(event EventTick
  (params (DeltaSeconds :type Float%20%28single-precision%29))
  (Development|PrintString (Utilities|String|ToString(Integer) (Utilities|Array|Length (Variables|Default|GetdeleteActorArray))) true true "(R=1.000000,G=0.000000,B=0.000000,A=1.000000)" DeltaSeconds)
  (for _array_element (Variables|Default|GetdeleteActorArray)
    (Utilities|IsValid _array_element
      (:Is%20Valid
        (if (Math|Vector|Equal(Vector) (Transformation|GetVelocity _array_element) "0, 0, 0" 0.0001)
          (Utilities|ActorDelete _array_element))))))

(fn ConstructionScript)