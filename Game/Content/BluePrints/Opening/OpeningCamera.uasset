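; Opening movie camera that plays a sequence of cuts from MovieParameter, each moving along a spline for a set time.
; Speed curves, normalised by their time and value ranges, drive spline distance; rotation comes from a follow-actor look-at with offset, or a rotation curve.
; Tick advances the timer, repeating cuts by loop count and optionally looping the sequence.
; An arrow-key debug mode switches cuts, scales or pauses playback, and prints status.
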(event EventBeginPlay
  (Variables|Default|SetArrayIndex 0)
  (for _array_element (Variables|Default|GetMovieParameter)
    (Utilities|SpeedGraphSetting (.speedcurve _array_element))
    (Utilities|RotationGraphSetting (.rotationcurve _array_element)))
  (Variables|Default|SetNowSpline (Default|GetSpline (.splineactor (Utilities|Array|Get(acopy) (Variables|Default|GetMovieParameter) (Variables|Default|GetArrayIndex))))))

(event EventTick
  (params (DeltaSeconds :type Float%20%28single-precision%29))
  (Variables|Default|SetDeltaSeconds DeltaSeconds)
  (Utilities|IsValid (Variables|Default|GetNowSpline)
    (:Is%20Valid
      (Variables|Default|Settimer (+ (* (Variables|Default|GetDeltaSeconds) (Variables|Default|GetDebug_SpeedMag)) (Variables|Default|Gettimer)))
      (|DebugPrint
        (:execute
          ;[1 1 1] 現在のスプラインの長さを超えたかどうか
          (if (> (Variables|Default|Gettimer) (.movetime (Utilities|Array|Get(acopy) (Variables|Default|GetMovieParameter) (Variables|Default|GetArrayIndex))))
            (Utilities|ResetSpline)
            (else
              (Utilities|SetCameraPosition))))))
    (:Is%20Not%20Valid
      (Development|PrintString "[OpeningCamera] SplineActor is NULL" true true "(R=1.000000,G=0.575000,B=0.000000,A=1.000000)" (Variables|Default|GetDeltaSeconds)))))

(event Input|KeyboardEvents|Right
  (params (Key :type Key%20Structure :default "None"))
  (:Pressed
    (if (Variables|Default|GetDebugMode)
      (if (Variables|Default|GetDebug_Ctrl)
        (Variables|Default|SetDebug_SpeedMag (* (Variables|Default|GetDebug_SpeedMag) 2.0))
        (else
          (Utilities|IncrimentIndex))))))

(event Input|KeyboardEvents|Left
  (params (Key :type Key%20Structure :default "None"))
  (:Pressed
    (if (Variables|Default|GetDebugMode)
      (if (Variables|Default|GetDebug_Ctrl)
        (Variables|Default|SetDebug_SpeedMag (/ (Variables|Default|GetDebug_SpeedMag) 2.0))
        (else
          (Utilities|DecrimentIndex))))))

(event Input|KeyboardEvents|RightCtrl
  (params (Key :type Key%20Structure :default "None"))
  (:Pressed
    (if (Variables|Default|GetDebugMode)
      (Variables|Default|SetDebug_Ctrl true)))
  (:Released
    (Variables|Default|SetDebug_Ctrl false)))

(event Input|KeyboardEvents|LeftCtrl
  (params (Key :type Key%20Structure :default "None"))
  (:Pressed
    (if (Variables|Default|GetDebugMode)
      (Variables|Default|SetDebug_Ctrl true)))
  (:Released
    (Variables|Default|SetDebug_Ctrl false)))

(event Input|KeyboardEvents|Down
  (params (Key :type Key%20Structure :default "None"))
  (:Pressed
    (if (Variables|Default|GetDebugMode)
      (if (Variables|Default|GetDebug_Ctrl)
        (Variables|Default|SetDebug_SpeedMag 1.0)
        (else
          (Variables|Default|Settimer 0.0)
          (Variables|Default|SetArrayIndex 0)
          (Variables|Default|SetNowSpline (Default|GetSpline (.splineactor (Utilities|Array|Get(acopy) (Variables|Default|GetMovieParameter))))))))))

(event Input|KeyboardEvents|Up
  (params (Key :type Key%20Structure :default "None"))
  (:Pressed
    (if (Variables|Default|GetDebug_Ctrl)
      (if (== (Variables|Default|GetDebugTempMag) 0.0)
        (Variables|Default|SetDebugTempMag (Variables|Default|GetDebug_SpeedMag))
        (Variables|Default|SetDebug_SpeedMag 0.0)
        (else
          (Variables|Default|SetDebug_SpeedMag (Variables|Default|GetDebugTempMag))
          (Variables|Default|SetDebugTempMag 0.0)))
      (else
        (bind _output_get (Variables|Default|SetDebugMode (not (Variables|Default|GetDebugMode))))
        (if (not _output_get)
          (Variables|Default|SetDisableHowToDebugModeTime 0.0))))))

(fn ConstructionScript
  (if (not (Variables|Debug|GetIsEnableHowToDebugMessage))
    (Variables|Default|SetHowToDebugModeMessage "")))