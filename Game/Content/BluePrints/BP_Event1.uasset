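; Scripted event actor that plays a girl-and-water hazard sequence when GameManager's active event count matches its EventNum.
; Tick opens BPDoor, lerps the girl to GirlGoal, then reveals and grows the water before clearing the event flag and destroying the girl.
; Live commentary lines queue once at the start and after the girl arrives.
; A BP_Chair touching the water gets a randomly angled forward vector and loses input for a few seconds.
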(event OnComponentBeginOverlap(Water)
  (params (OverlappedComponent :type Primitive%20Component%20Object%20Reference) (OtherActor :type Actor%20Object%20Reference) (OtherComp :type Primitive%20Component%20Object%20Reference) (OtherBodyIndex :type Integer) (bFromSweep :type Boolean) (SweepResult :type Hit%20Result%20Structure%20%28by%20ref%29))
  (bind _returnvalue (Math|Random|RandomFloatinRange -5.0 -15.0))
  (bind _returnvalue_2 (Math|Trig|DegreesToRadians _returnvalue))
  (bind _asbp_chair (Utilities|Casting|CastToBP_Chair OtherActor))
  (Variables|Default|Setis_entry true)
  (if (Math|Random|RandomBool)
    _
    (else
      _))
  (Class|Chair|SetForwardVec _asbp_chair (Math|Vector|MakeVector (Math|Trig|Cos(Radians) _returnvalue_2) (Math|Trig|Sin(Radians) _returnvalue_2) 0.0))
  (Variables|/Script/Chase.Chair|Setm_can_input_ _asbp_chair false)
  (Utilities|FlowControl|Delay 3.0)
  (Variables|/Script/Chase.Chair|Setm_can_input_ _asbp_chair true))

(event EventBeginPlay
  (Variables|Default|Setstartlocation (Transformation|GetWorldLocation (Variables|Default|GetBP_Girl)))
  (bind _output_get (Variables|Default|Setdef_scale (Variables|/Script/Engine.SceneComponent|GetRelativeScale3D (Variables|Default|GetWater))))
  (Variables|Default|Setmax_scale (Math|Vector|MakeVector (.x (Variables|Default|Getmax_scale)) (.y (Variables|Default|Getmax_scale)) (.z _output_get)))
  (Rendering|SetVisibility (Variables|Default|GetWater) false false)
  (Rendering|SetVisibility (Variables|Default|GetBP_Girl) false true))

(event Collision|EventActorBeginOverlap
  (params (OtherActor :type Actor%20Object%20Reference)))

(event EventTick
  (params (DeltaSeconds :type Float%20%28single-precision%29))
  (bind _bp_door (Variables|Default|GetBP_Door))
  (bind _girlgoal (Variables|Default|GetGirlGoal))
  (bind _startlocation (Variables|Default|Getstartlocation))
  (bind _gamemanager (Variables|Default|GetGameManager))
  (bind _returnvalue (Transformation|GetWorldLocation _girlgoal))
  (if (and (Variables|/Script/Chase.GameManager|Getm_is_event_ _gamemanager) (== (Variables|/Script/Chase.GameManager|Getm_event_cnt_ _gamemanager) (Variables|Default|Getevent_num)))
    (Rendering|SetVisibility (Variables|Default|GetBP_Girl) true true)
    (Utilities|FlowControl|Sequence
      (:then_0
        (Utilities|FlowControl|DoOnce false
          (:Completed
            (Utilities|LiveComment "LC_8_1"))))
      (:then_1
        (Variables|/Game/BluePrints/BP_Door.BP_Door_C|SetIs_Move _bp_door true)
        (if (Variables|/Game/BluePrints/BP_Door.BP_Door_C|GetMove_End _bp_door)
          (Transformation|SetWorldLocation (Variables|Default|GetBP_Girl) (Math|Vector|Lerp(Vector) (Math|Vector|MakeVector (.x _startlocation) (.y _startlocation) (.z _startlocation)) (Math|Vector|MakeVector (.x _returnvalue) (.y _returnvalue) (.z _returnvalue)) (Variables|Default|Getmove_alpha)) false true)
          (if (< (+ (Variables|Default|Getmove_alpha) (* (Variables|Default|Getmove_speed) DeltaSeconds)) 1.0)
            (Variables|Default|Setmove_alpha (+ (Variables|Default|Getmove_alpha) (* (Variables|Default|Getmove_speed) DeltaSeconds)))
            (else
              (Utilities|FlowControl|Sequence
                (:then_0
                  (Variables|Default|Setmove_alpha 1.0)
                  (Rendering|SetVisibility (Variables|Default|GetWater) true false)
                  (Transformation|SetRelativeScale3D (Variables|Default|GetWater) (Math|Vector|Lerp(Vector) (Variables|Default|Getdef_scale) (Variables|Default|Getmax_scale) (Variables|Default|Getscale_alpha)))
                  (if (< (+ (Variables|Default|Getscale_alpha) (* (Variables|Default|Getscale_speed) DeltaSeconds)) 1.0)
                    (Variables|Default|Setscale_alpha (+ (Variables|Default|Getscale_alpha) (* (Variables|Default|Getscale_speed) DeltaSeconds)))
                    (else
                      (Variables|Default|Setscale_alpha 1.0)
                      (Utilities|FlowControl|Delay 3.0)
                      (Variables|/Script/Chase.GameManager|Setm_is_event_ (Variables|Default|GetGameManager) false)
                      (Utilities|FlowControl|Delay 2.0)
                      (Components|DestroyComponent (Variables|Default|GetBP_Girl)))))
                (:then_1
                  (Utilities|FlowControl|DoOnce false
                    (:Completed
                      (Utilities|LiveComment "LC_8_2")
                      (Utilities|LiveComment "C_8"))))))))))))

(fn ConstructionScript
  (bind _returnvalue (Rendering|Material|CreateDynamicMaterialInstance (Variables|Default|GetWater) 0 "/Game/Materials/M_SimpleWater.M_SimpleWater" "None" :!class /Script/Engine.PrimitiveComponent))
  (Variables|Default|SetWater_Mat _returnvalue))