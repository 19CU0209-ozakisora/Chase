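; BP_Chair is a chair pawn that slides as a physics object, with phase-driven behavior.
; On BeginPlay, chairs flagged IsMovement jump to the end phase, drop their arrow and simulate physics constrained to the XY plane.
; Tick enables physics during the slip phase, and Q feeds a fixed X-axis vector to the floating movement component.
; Hit handling and self-possession are disconnected; a note says hit logic moved to C++.
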(event EventBeginPlay
  ;[1 1 1] 操作(予定)の椅子なら入力受け付けにする、それ以外ならもろもろの設定
  (Transformation|SetWorldScale3D (Variables|Default|GetCamera) "1.000000,1.000000,1.000000")
  (if (Variables|Default|Getis_movement_)
    (Variables|Default|Setphase_ "kEnd")
    (Components|DestroyComponent (Variables|Default|Getm_parrow_))
    (Physics|SetSimulatePhysics (Variables|Default|Getm_pplayermesh_) true)
    (Class|PrimitiveComponent|SetConstraintMode (Variables|Default|Getm_pplayermesh_) "XYPlane")))

(event EventTick
  (params (DeltaSeconds :type Float%20%28single-precision%29))
  ;[1 1 1] 滑ってる時は物理挙動ON
  (if (Utilities|Enum|Equal(Enum) (Variables|Default|Getphase_) "kSlip")
    (Physics|SetSimulatePhysics (Variables|Default|Getm_pplayermesh_) true)))

(event Input|KeyboardEvents|Q
  (params (Key :type Key%20Structure :default "None"))
  (:Pressed
    (Class|PawnMovementComponent|AddInputVector (Variables|Default|Getm_floating_pawn_movement_) "500.000000, 0, 0" false)))

(fn ConstructionScript)