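; powerChair is an actor that acts as a visual power indicator for a referenced chair Blueprint.
; Each tick, it shows its static mesh only while the chair accepts input and is in the KPowerChange phase.
; It also slides the mesh along local X by the absolute Y input value times DistanceScale, leaving Y and Z unchanged.
; An actor-scaling node is left unconnected and never runs.
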(event EventTick
  (params (DeltaSeconds :type Float%20%28single-precision%29))
  (bind _staticmesh (Variables|Default|GetStaticMesh))
  (bind _chairbp (Variables|Default|GetChairBP))
  (bind _relativelocation (Variables|/Script/Engine.SceneComponent|GetRelativeLocation _staticmesh))
  (Utilities|IsValid _chairbp
    (:Is%20Valid
      (Rendering|SetVisibility (Variables|Default|GetStaticMesh) (and (Variables|/Script/Chase.Chair|Getm_can_input_ _chairbp) (Utilities|Enum|Equal(Enum) (Class|Chair|GetPhase (Variables|Default|GetChairBP)) "kPowerChange")) true)
      (Transformation|SetRelativeLocation _staticmesh (Math|Vector|MakeVector (* (Math|Float|Absolute(Float) (.y (Variables|/Script/Chase.Chair|Getm_input_value_ (Variables|Default|GetChairBP)))) (Variables|Default|GetDistanceScale)) (.y _relativelocation) (.z _relativelocation)) false false))))

(fn ConstructionScript)