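; Stage camera actor that glides its camera from the start position to the actor's root, driving round flow through the Gamemanager.
; Tick runs a delayed intro move that enables the current chair's input, then flag-triggered moves that call NextRound and snap back.
; CameraMove lerps by an accumulated Alpha, with separate intro, event-round and default speeds.
; EventTrigger overlaps on event rounds set MIsEvent, pausing movement, and increment the event count.
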(event OnComponentBeginOverlap(EventTrigger)
  (params (OverlappedComponent :type Primitive%20Component%20Object%20Reference) (OtherActor :type Actor%20Object%20Reference) (OtherComp :type Primitive%20Component%20Object%20Reference) (OtherBodyIndex :type Integer) (bFromSweep :type Boolean) (SweepResult :type Hit%20Result%20Structure%20%28by%20ref%29))
  (bind _gamemanager (Variables|Default|Getgamemanager))
  ;[1 1 1] 現在のターン数が特定のターンだった時フラグを立てる
  (if (Actor|ActorHasTag OtherActor "StageCamera")
    (CallFunction|EventCheck)
    (if (Variables|Default|Getcheck_flag)
      (Variables|/Script/Chase.GameManager|Setm_is_event_ _gamemanager true)
      (bind _result (Math|Integer|IncrementInt (Variables|/Script/Chase.GameManager|Getm_event_cnt_ _gamemanager))
        (:%20%20
          (Variables|/Script/Chase.GameManager|Setm_event_cnt_ _gamemanager _result))))))

(event EventBeginPlay
  (Variables|Default|Setstart_location (Transformation|GetWorldLocation (Variables|CameraActor|GetCameraComponent)))
  (Variables|Default|Setgoal_location (Transformation|GetWorldLocation (Variables|Default|GetScene))))

(event Collision|EventActorBeginOverlap
  (params (OtherActor :type Actor%20Object%20Reference)))

(event EventTick
  (params (DeltaSeconds :type Float%20%28single-precision%29))
  (bind _gamemanager (Variables|Default|Getgamemanager))
  (if (Variables|Default|Getonce)
    (bind _output_get (Variables|Default|Settime_cnt (+ (Variables|Default|Gettime_cnt) DeltaSeconds)))
    (if (>= _output_get (Variables|Default|Getdelay_time))
      (CallFunction|CameraMove DeltaSeconds)
      (if (== (Variables|Default|Getalpha) 1.0)
        (Utilities|FlowControl|Delay 5.0)
        (Variables|Default|Setonce false)
        (Variables|/Script/Chase.Chair|Setm_can_input_ (Utilities|Array|Get(acopy) (Variables|/Script/Chase.GameManager|Getm_chairs_ _gamemanager) (- (Variables|/Script/Chase.GameManager|Getm_nowroundnum_ _gamemanager) 1)) true)))
    (elif (not (Variables|/Script/Chase.GameManager|Getm_is_event_ (Variables|Default|Getgamemanager)))
      (if (Variables|Default|Getmove_flag)
        (CallFunction|CameraMove DeltaSeconds)
        (if (== (Variables|Default|Getalpha) 1.0)
          (Utilities|FlowControl|Delay 3.0)
          (Class|GameManager|NextRound (Variables|Default|Getgamemanager))
          (CallFunction|ResetCameraLocation))))))

(fn ConstructionScript)

(fn CameraMove
  (params (B :type Float%20%28single-precision%29))
  (Transformation|SetWorldLocation (Variables|CameraActor|GetCameraComponent) (Math|Vector|Lerp(Vector) (Variables|Default|Getstart_location) (Variables|Default|Getgoal_location) (Variables|Default|Getalpha)) false false)
  (if (Variables|Default|Getonce)
    (Variables|Default|Setalpha (+ (Variables|Default|Getalpha) (* (Variables|Default|Getfirst_speed) B)))
    (if (> (Variables|Default|Getalpha) 1.0)
      (Variables|Default|Setalpha 1.0))
    (else
      (CallFunction|EventCheck)
      (if (Variables|Default|Getcheck_flag)
        (Variables|Default|Setalpha (+ (Variables|Default|Getalpha) (* (Variables|Default|Getevent_speed) B)))
        (if (> (Variables|Default|Getalpha) 1.0)
          (Variables|Default|Setalpha 1.0))
        (else
          (Variables|Default|Setalpha (+ (Variables|Default|Getalpha) (* (Variables|Default|Getdefault_speed) B)))
          (if (> (Variables|Default|Getalpha) 1.0)
            (Variables|Default|Setalpha 1.0)))))))

(fn ResetCameraLocation
  (Transformation|SetWorldLocation (Variables|CameraActor|GetCameraComponent) (Variables|Default|Getstart_location) false true)
  (Variables|Default|Setalpha 0.0)
  (Variables|Default|Setcheck_flag false)
  (Variables|Default|Setmove_flag false))

(fn EventCheck
  (bind _gamemanager (Variables|Default|Getgamemanager))
  (bind _array_element (Utilities|Array|ForEachLoopwithBreak (Variables|/Script/Chase.GameManager|Getm_event_round_ _gamemanager) :!label _label)
    (:LoopBody
      (if (== _array_element (Variables|/Script/Chase.GameManager|Getm_nowroundnum_ _gamemanager))
        (Variables|Default|Setcheck_flag true)
        (goto _label Break)))))