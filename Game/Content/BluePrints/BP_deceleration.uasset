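; BP_deceleration is a trigger actor that brakes a Chair pawn to a stop once it overlaps the collision component.
; Overlap stores the Chair and sets a deceleration flag, unless the overlapped component is tagged "targetpoint".
; Tick then lowers the floating movement's MaxSpeed at a frame-rate-independent rate, printing it for debugging.
; When speed runs out, it zeroes MaxSpeed, sets the Chair's phase to KEnd and clears the flag.
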(event OnComponentBeginOverlap(CollisionComponent)
  (params (OverlappedComponent :type Primitive%20Component%20Object%20Reference) (OtherActor :type Actor%20Object%20Reference) (OtherComp :type Primitive%20Component%20Object%20Reference) (OtherBodyIndex :type Integer) (bFromSweep :type Boolean) (SweepResult :type Hit%20Result%20Structure%20%28by%20ref%29))
  (if (not (Components|ComponentHasTag OverlappedComponent "targetpoint"))
    (bind _aschair (Utilities|Casting|CastToChair OtherActor))
    (Variables|Default|Setdeceleration_chair_ _aschair)
    (Variables|Default|Setdeceleration_flag_ true)))

(event EventBeginPlay)

(event EventTick
  (params (DeltaSeconds :type Float%20%28single-precision%29))
  (bind _deceleration_chair_ (Variables|Default|Getdeceleration_chair_))
  (bind _deceleration_val_ (Variables|Default|Getdeceleration_val_))
  (bind _returnvalue (* _deceleration_val_ DeltaSeconds))
  (bind _m_floating_pawn_movement_ (Variables|/Script/Chase.Chair|Getm_floating_pawn_movement_ _deceleration_chair_))
  (if (Variables|Default|Getdeceleration_flag_)
    (Utilities|IsValid _deceleration_chair_
      (:Is%20Valid
        (if (>= (Variables|/Script/Engine.FloatingPawnMovement|GetMaxSpeed _m_floating_pawn_movement_) _returnvalue)
          (bind _output_get (Variables|/Script/Engine.FloatingPawnMovement|SetMaxSpeed _m_floating_pawn_movement_ (- (Variables|/Script/Engine.FloatingPawnMovement|GetMaxSpeed _m_floating_pawn_movement_) _returnvalue)))
          (Development|PrintString (Utilities|String|ToString(Float) _output_get) true true "(R=0.000000,G=0.660000,B=1.000000,A=1.000000)" DeltaSeconds)
          (else
            (Variables|/Script/Engine.FloatingPawnMovement|SetMaxSpeed _m_floating_pawn_movement_ 0.0)
            (Class|Chair|SetPhase _deceleration_chair_ "kEnd")
            (Variables|Default|Setdeceleration_flag_ false)))))))

(fn ConstructionScript)