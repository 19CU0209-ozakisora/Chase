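; Double door actor that swings open or closed when a BP_Chair overlaps its open or close trigger.
; Each trigger sets a flag that makes Tick step a time value forward or back, with Speed multiplying the whole updated time.
; DoorCurve converts that time into mirrored world-space yaw for both leaves, with FrontOpen choosing the swing direction.
; A separate ResetRotation function zeroes both leaves' world rotation.
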(event OnComponentBeginOverlap(OpenTrigger)
  (params (OverlappedComponent :type Primitive%20Component%20Object%20Reference) (OtherActor :type Actor%20Object%20Reference) (OtherComp :type Primitive%20Component%20Object%20Reference) (OtherBodyIndex :type Integer) (bFromSweep :type Boolean) (SweepResult :type Hit%20Result%20Structure%20%28by%20ref%29))
  (Utilities|Casting|CastToBP_Chair OtherActor)
  (Variables|Default|SetOpenFlag true))

(event OnComponentBeginOverlap(CloseTrigger)
  (params (OverlappedComponent :type Primitive%20Component%20Object%20Reference) (OtherActor :type Actor%20Object%20Reference) (OtherComp :type Primitive%20Component%20Object%20Reference) (OtherBodyIndex :type Integer) (bFromSweep :type Boolean) (SweepResult :type Hit%20Result%20Structure%20%28by%20ref%29))
  (Utilities|Casting|CastToBP_Chair OtherActor)
  (Variables|Default|SetCloseFlag true))

(event EventTick
  (params (DeltaSeconds :type Float%20%28single-precision%29))
  (Utilities|FlowControl|Sequence
    (:then_0
      ;[1 1 1] 開く時の処理
      (if (Variables|Default|GetOpenFlag)
        (if (< (Variables|Default|GetTime) (.MaxTime (Math|Curves|GetTimeRange (Variables|Default|GetDoor_Curve))))
          (bind _output_get (Variables|Default|SetTime (* (+ (Variables|Default|GetTime) DeltaSeconds) (Variables|Default|GetSpeed))))
          (if (Variables|Default|GetFrontOpen)
            (Transformation|SetWorldRotation (Variables|Default|GetRightDoor) (Math|Rotator|MakeRotator 0.0 0.0 (Math|Curves|GetFloatValue (Variables|Default|GetDoor_Curve) _output_get)) false false)
            (Transformation|SetWorldRotation (Variables|Default|GetLeftDoor) (Math|Rotator|MakeRotator 0.0 0.0 (* (Math|Curves|GetFloatValue (Variables|Default|GetDoor_Curve) _output_get) -1.0)) false false)
            (else
              (Transformation|SetWorldRotation (Variables|Default|GetRightDoor) (Math|Rotator|MakeRotator 0.0 0.0 (* (Math|Curves|GetFloatValue (Variables|Default|GetDoor_Curve) _output_get) -1.0)) false false)
              (Transformation|SetWorldRotation (Variables|Default|GetLeftDoor) (Math|Rotator|MakeRotator 0.0 0.0 (Math|Curves|GetFloatValue (Variables|Default|GetDoor_Curve) _output_get)) false false)))
          (else
            (Variables|Default|SetTime 1.0)
            (Variables|Default|SetOpenFlag false)))))
    (:then_1
      ;[1 1 1] 閉じる時の処理
      (if (Variables|Default|GetCloseFlag)
        (if (> (Variables|Default|GetTime) (.MinTime (Math|Curves|GetTimeRange (Variables|Default|GetDoor_Curve))))
          (bind _output_get_2 (Variables|Default|SetTime (* (- (Variables|Default|GetTime) DeltaSeconds) (Variables|Default|GetSpeed))))
          (if (Variables|Default|GetFrontOpen)
            (Transformation|SetWorldRotation (Variables|Default|GetRightDoor) (Math|Rotator|MakeRotator 0.0 0.0 (Math|Curves|GetFloatValue (Variables|Default|GetDoor_Curve) _output_get_2)) false false)
            (Transformation|SetWorldRotation (Variables|Default|GetLeftDoor) (Math|Rotator|MakeRotator 0.0 0.0 (* (Math|Curves|GetFloatValue (Variables|Default|GetDoor_Curve) _output_get_2) -1.0)) false false)
            (else
              (Transformation|SetWorldRotation (Variables|Default|GetRightDoor) (Math|Rotator|MakeRotator 0.0 0.0 (* (Math|Curves|GetFloatValue (Variables|Default|GetDoor_Curve) _output_get_2) -1.0)) false false)
              (Transformation|SetWorldRotation (Variables|Default|GetLeftDoor) (Math|Rotator|MakeRotator 0.0 0.0 (Math|Curves|GetFloatValue (Variables|Default|GetDoor_Curve) _output_get_2)) false false)))
          (else
            (Variables|Default|SetTime 0.0)
            (Variables|Default|SetCloseFlag false)))))))

(fn ConstructionScript)

(fn ResetRotation
  (Transformation|SetWorldRotation (Variables|Default|GetRightDoor) "0, 0, 0" false false)
  (Transformation|SetWorldRotation (Variables|Default|GetLeftDoor) "0, 0, 0" false false))