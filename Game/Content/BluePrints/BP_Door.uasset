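; BP_Door is a door actor that slides its left mesh along relative X, following a float curve.
; BeginPlay caches the mesh's starting location.
; While IsMove is true, Tick accumulates time and adds the curve value to that starting X, then sets MoveEnd once the curve's time range is exceeded.
; Nothing here sets IsMove or resets the timer.
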(event EventBeginPlay
  (Variables|Default|SetDef_Location (Variables|/Script/Engine.SceneComponent|GetRelativeLocation (Variables|Default|Getm_pdoor_mesh_left_))))

(event Collision|EventActorBeginOverlap
  (params (OtherActor :type Actor%20Object%20Reference)))

(event EventTick
  (params (DeltaSeconds :type Float%20%28single-precision%29))
  (bind _def_location (Variables|Default|GetDef_Location))
  (if (Variables|Default|GetIs_Move)
    (if (< (Variables|Default|GetTime) (.MaxTime (Math|Curves|GetTimeRange (Variables|Default|GetDoor_Curve))))
      (bind _output_get (Variables|Default|SetTime (+ DeltaSeconds (Variables|Default|GetTime))))
      (Transformation|SetRelativeLocation (Variables|Default|Getm_pdoor_mesh_left_) (Math|Vector|MakeVector (+ (.x _def_location) (Math|Curves|GetFloatValue (Variables|Default|GetDoor_Curve) _output_get)) (.y _def_location) (.z _def_location)) false false)
      (else
        (Variables|Default|SetMove_End true)))))

(fn ConstructionScript)