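; Stage event where two mop boys clean up BP_Event1's water, triggered when GameManager's active event count matches EventNum.
; Tick reveals and lerps the boys to their goals with live commentary, then fades the water material's opacity, shows a shine effect and ends the event.
; Afterwards, Water overlaps knock a BP_Chair onto a random angled heading with input briefly disabled, and SpeedUP overlaps multiply its projectile velocity.
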(event OnComponentBeginOverlap(Water)
  (params (OverlappedComponent :type Primitive%20Component%20Object%20Reference) (OtherActor :type Actor%20Object%20Reference) (OtherComp :type Primitive%20Component%20Object%20Reference) (OtherBodyIndex :type Integer) (bFromSweep :type Boolean) (SweepResult :type Hit%20Result%20Structure%20%28by%20ref%29))
  (bind _returnvalue (Math|Random|RandomFloatinRange -5.0 -15.0))
  (bind _returnvalue_2 (Math|Trig|DegreesToRadians _returnvalue))
  (if (Variables|Default|Getis_event_end)
    (bind _asbp_chair (Utilities|Casting|CastToBP_Chair OtherActor))
    (Variables|Default|Setis_entry true)
    (if (Math|Random|RandomBool)
      _
      (else
        _))
    (Class|Chair|SetForwardVec _asbp_chair (Math|Vector|MakeVector (Math|Trig|Cos(Radians) _returnvalue_2) (Math|Trig|Sin(Radians) _returnvalue_2) 0.0))
    (Variables|/Script/Chase.Chair|Setm_can_input_ _asbp_chair false)
    (Utilities|FlowControl|Delay 3.0)
    (Variables|/Script/Chase.Chair|Setm_can_input_ _asbp_chair true)))

(event OnComponentBeginOverlap(SpeedUP)
  (params (OverlappedComponent :type Primitive%20Component%20Object%20Reference) (OtherActor :type Actor%20Object%20Reference) (OtherComp :type Primitive%20Component%20Object%20Reference) (OtherBodyIndex :type Integer) (bFromSweep :type Boolean) (SweepResult :type Hit%20Result%20Structure%20%28by%20ref%29))
  (if (Variables|Default|Getis_event_end)
    (bind _asbp_chair (Utilities|Casting|CastToBP_Chair OtherActor))
    (Variables|/Script/Engine.MovementComponent|SetVelocity (Variables|/Script/Chase.Chair|Getm_projectile_movement_ _asbp_chair) (* (Variables|/Script/Engine.MovementComponent|GetVelocity (Variables|/Script/Chase.Chair|Getm_projectile_movement_ _asbp_chair)) (Variables|Default|Getspeedup_scale)))))

(event EventBeginPlay
  (bind _bp_event1 (Variables|Default|GetBP_Event1))
  (Variables|Default|Setstartlocation (Utilities|Array|MakeArray (Transformation|GetWorldLocation (Variables|Default|GetBP_Mop_Boy1)) (Transformation|GetWorldLocation (Variables|Default|GetBP_Mop_Boy2))))
  (Variables|Default|Setgoallocation (Utilities|Array|MakeArray (Transformation|GetWorldLocation (Variables|Default|GetBoy_1_Goal)) (Transformation|GetWorldLocation (Variables|Default|GetBoy_2_Goal))))
  (Rendering|SetVisibility (Variables|Default|GetBP_Mop_Boy1) false true)
  (Rendering|SetVisibility (Variables|Default|GetBP_Mop_Boy2) false true)
  (bind _output_get (Variables|Default|Setdef_scale (* (Variables|/Game/BluePrints/BP_Event1.BP_Event1_C|Getmax_scale _bp_event1) (Transformation|GetWorldScale (Variables|/Game/BluePrints/BP_Event1.BP_Event1_C|GetBP_Girl _bp_event1)))))
  (bind _output_get_2 (Variables|Default|Setreduction_scale (Math|Vector|MakeVector (.x _output_get) (.y (/ (Math|Vector|MakeVector 1.0 (.y _output_get) 1.0) 3.0)) (.z _output_get))))
  (Rendering|SetVisibility (Variables|Default|GetShine_EF) false false))

(event Collision|EventActorBeginOverlap
  (params (OtherActor :type Actor%20Object%20Reference)))

(event EventTick
  (params (DeltaSeconds :type Float%20%28single-precision%29))
  (bind _bp_event1 (Variables|Default|GetBP_Event1))
  (bind _gamemanager (Variables|Default|GetGameManager))
  (bind _water_mat (Variables|/Game/BluePrints/BP_Event1.BP_Event1_C|GetWater_Mat _bp_event1))
  (if (and (Variables|/Script/Chase.GameManager|Getm_is_event_ _gamemanager) (== (Variables|/Script/Chase.GameManager|Getm_event_cnt_ _gamemanager) (Variables|Default|Getevent_num)))
    (Rendering|SetVisibility (Variables|Default|GetBP_Mop_Boy1) true true)
    (Utilities|FlowControl|Sequence
      (:then_0
        (Utilities|FlowControl|DoOnce false
          (:Completed
            (Utilities|LiveComment "LC_9")
            (Utilities|LiveComment "C_9"))))
      (:then_1
        (Rendering|SetVisibility (Variables|Default|GetBP_Mop_Boy2) true true)
        (for (_array_element _array_index) (Variables|Default|Getstartlocation)
          (if (== _array_index 0)
            (Transformation|SetWorldLocation (Variables|Default|GetBP_Mop_Boy1) (Math|Vector|Lerp(Vector) (Math|Vector|MakeVector (.x _array_element) (.y _array_element) (.z _array_element)) (Math|Vector|MakeVector (.x (Utilities|Array|Get(acopy) (Variables|Default|Getgoallocation) _array_index)) (.y (Utilities|Array|Get(acopy) (Variables|Default|Getgoallocation) _array_index)) (.z _array_element)) (Variables|Default|Getmove_alpha)) false true)
            (else
              (Transformation|SetWorldLocation (Variables|Default|GetBP_Mop_Boy2) (Math|Vector|Lerp(Vector) (Math|Vector|MakeVector (.x _array_element) (.y _array_element) (.z _array_element)) (Math|Vector|MakeVector (.x (Utilities|Array|Get(acopy) (Variables|Default|Getgoallocation) _array_index)) (.y (Utilities|Array|Get(acopy) (Variables|Default|Getgoallocation) _array_index)) (.z _array_element)) (Variables|Default|Getmove_alpha)) false true)))
          (if (< (+ (Variables|Default|Getmove_alpha) (* (Variables|Default|Getmove_speed) DeltaSeconds)) 1.0)
            (Variables|Default|Setmove_alpha (+ (Variables|Default|Getmove_alpha) (* (Variables|Default|Getmove_speed) DeltaSeconds)))
            (else
              (Variables|Default|Setmove_alpha 1.0)
              ;[1 1 1] ふとうめいど
              (bind _returnvalue (Rendering|Material|GetScalarParameterValue _water_mat "opacity" :!class /Script/Engine.MaterialInstanceDynamic))
              (Rendering|Material|SetScalarParameterValue _water_mat "opacity" (- _returnvalue (* DeltaSeconds (Variables|Default|Getreduction))) :!class /Script/Engine.MaterialInstanceDynamic)
              (if (< (- _returnvalue (* DeltaSeconds (Variables|Default|Getreduction))) 0.0)
                (Rendering|SetVisibility (Variables|Default|GetShine_EF) true false)
                (Utilities|FlowControl|Delay 3.0)
                (Variables|/Script/Chase.GameManager|Setm_is_event_ (Variables|Default|GetGameManager) false)
                (Variables|Default|Setis_event_end true)))))))))

(fn ConstructionScript)