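; BP_GameManager is an actor that sets up the on-screen point display for players 1P and 2P.
; On BeginPlay it creates one BP_PointWidget_1P, stores it as both 1PPoint and 2PPoint, and adds it to the viewport.
; It passes itself to that widget as both GameManager and GameManager02.
; Nodes that would copy GetPoint1P and GetPoint2P results into the widget are unconnected and never run.
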(event EventBeginPlay
  (bind _returnvalue (UserInterface|CreateWidget "/Game/BluePrints/BP_PointWidget_1P.BP_PointWidget_1P_C"))
  (Variables|Default|Set1P_Point _returnvalue)
  (Variables|/Game/BluePrints/BP_PointWidget_1P.BP_PointWidget_1P_C|SetGameManager (Variables|Default|Get1P_Point) self)
  (Variables|Default|Set2P_Point _returnvalue)
  (UserInterface|Viewport|AddtoViewport _returnvalue 0)
  (Variables|/Game/BluePrints/BP_PointWidget_1P.BP_PointWidget_1P_C|SetGameManager02 (Variables|Default|Get2P_Point) self))

(event Collision|EventActorBeginOverlap
  (params (OtherActor :type Actor%20Object%20Reference)))

(event EventTick
  (params (DeltaSeconds :type Float%20%28single-precision%29)))

(fn ConstructionScript)