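; BP_Playerchara acts as a chair spawner, creating a BP_Chair at its Scene component's transform on BeginPlay and keeping a reference to it.
; Tick polls that chair's Phase; at 3, it waits five seconds through a Delay, then spawns and tracks a new chair without destroying the old one.
; Debug strings report spawn validity and the wait, while a printed countdown chain is left unconnected.
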(event EventBeginPlay
  (bind _returnvalue (Game|SpawnActorfromClass "/Game/BluePrints/BP_Chair.BP_Chair_C" (Transformation|GetWorldTransform (Variables|Default|GetScene)) "Undefined" 0 0))
  (bind _output_get (Variables|Default|SetChair _returnvalue))
  (Utilities|IsValid _output_get
    (:Is%20Valid
      (Development|PrintString "T"))
    (:Is%20Not%20Valid
      (Development|PrintString "F"))))

(event Collision|EventActorBeginOverlap
  (params (OtherActor :type Actor%20Object%20Reference)))

(event EventTick
  (params (DeltaSeconds :type Float%20%28single-precision%29))
  (if (== (Variables|/Script/Chase.Chair|Getphase_ (Variables|Default|GetChair)) 3)
    (Development|PrintString "5" true false "(R=0.000000,G=0.660000,B=1.000000,A=1.000000)" DeltaSeconds)
    (Utilities|FlowControl|Delay 5.0)
    (bind _returnvalue (Game|SpawnActorfromClass "/Game/BluePrints/BP_Chair.BP_Chair_C" (Transformation|GetWorldTransform (Variables|Default|GetScene)) "Undefined" 0 0))
    (Variables|Default|SetChair _returnvalue)))

(fn ConstructionScript)