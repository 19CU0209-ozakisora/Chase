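; BP_Player is the player Blueprint that spawns chairs and hands player control over to them.
; CreateChair spawns a BP_Chair at the ChairSpawner transform, stores it as ControlChair and calls SetChairTag.
; GetOperate teleports that chair to the player's location, sets its phase to KMove and has player controller 0 possess it.
; Tick is empty, with comments noting its logic moved to the C++ GameManager; leftover respawn and debug nodes are disconnected.
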(event EventGetOperate
  (bind _control_chair_ (Variables|Default|Getcontrol_chair_))
  (Transformation|SetActorLocation _control_chair_ (Transformation|GetActorLocation) false true)
  (Variables|/Script/Chase.Chair|Setm_phase_ _control_chair_ "kMove")
  (Pawn|Possess (Game|GetPlayerController 0) _control_chair_))

(event Collision|EventActorBeginOverlap
  (params (OtherActor :type Actor%20Object%20Reference)))

(event EventTick
  (params (DeltaSeconds :type Float%20%28single-precision%29))
  ;[1 1 1] (05/07にGameManager C++に移植済み)
)

(event EventCreateChair
  (bind _returnvalue (Game|SpawnActorfromClass "/Game/BluePrints/BP_Chair.BP_Chair_C" (Transformation|GetWorldTransform (Variables|Default|Getchair_spawner_)) "Undefined" 0 0))
  (Variables|Default|Setcontrol_chair_ _returnvalue)
  (Class|Playerchara|SetChairTag))

(fn ConstructionScript)